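; FastF_BP is a comic bubble prop whose plane shows or hides based on how close pawns are.
; BeginPlay sets the plane's initial visibility from StartVisible.
; Each Tick runs two sphere overlaps: a pawn within ScanRange, or StartVisible, shows the plane, while one within a smaller fixed radius sets Hidden, which overrides both.
; Hidden updates after visibility is applied, so it takes effect the following tick.
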(event EventBeginPlay
  (Rendering|SetVisibility (Variables|Default|GetPlane) (Variables|Default|GetStart%20visible) false))

(event Collision|EventActorBeginOverlap
  (params (OtherActor :type Actor%20Object%20Reference)))

(event EventTick
  (params (DeltaSeconds :type Float%20%28single-precision%29))
  (Utilities|FlowControl|Sequence
    (:then_0
      (bind _returnvalue (Collision|SphereOverlapActors (Transformation|GetActorLocation) (Variables|Default|GetScanRange) (Utilities|Array|MakeArray "ObjectTypeQuery3") "/Script/Engine.Actor"))
      (Rendering|SetVisibility (Variables|Default|GetPlane) (and (or _returnvalue (Variables|Default|GetStart%20visible)) (not (Variables|Default|GetHidden))) false))
    (:then_1
      (bind _returnvalue_2 (Collision|SphereOverlapActors (Transformation|GetActorLocation) 2e+02 (Utilities|Array|MakeArray "ObjectTypeQuery3") "/Script/Engine.Actor"))
      (Variables|Default|SetHidden _returnvalue_2))))

(fn ConstructionScript)