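; Elevator prop Blueprint that raises a cube platform while a pawn stands in its trigger box.
; Box overlap plays a timeline after a short delay, lerping the cube's relative Z from zero up to a configurable height.
; Ending the overlap reverses the timeline, first waiting a configurable hold time unless the position is flagged as fixed.
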(event OnComponentBeginOverlap(Box)
  (params (OverlappedComponent :type Primitive%20Component%20Object%20Reference) (OtherActor :type Actor%20Object%20Reference) (OtherComp :type Primitive%20Component%20Object%20Reference) (OtherBodyIndex :type Integer) (bFromSweep :type Boolean) (SweepResult :type Hit%20Result%20Structure%20%28by%20ref%29))
  (Utilities|Casting|CastToPawn OtherActor)
  (Utilities|FlowControl|Delay 0.2)
  (bind _elevator (Timeline|时间轴 Play)
    (:Update
      (Transformation|SetRelativeLocation (Variables|Default|GetCube) (Math|Vector|MakeVector 0.0 0.0 (Math|Float|Lerp 0.0 (Variables|Default|GetHigh%20value) _elevator)) false false))))

(event OnComponentEndOverlap(Box)
  (params (OverlappedComponent :type Primitive%20Component%20Object%20Reference) (OtherActor :type Actor%20Object%20Reference) (OtherComp :type Primitive%20Component%20Object%20Reference) (OtherBodyIndex :type Integer))
  (if (Variables|Default|GetFixed%20position)
    _
    (else
      (Utilities|FlowControl|Delay (Variables|Default|Getkeep%20position%20End%20time))))
  (Utilities|Casting|CastToPawn OtherActor)
  (Utilities|FlowControl|Delay 0.2)
  (bind _elevator (Timeline|时间轴 Reverse)
    (:Update
      (Transformation|SetRelativeLocation (Variables|Default|GetCube) (Math|Vector|MakeVector 0.0 0.0 (Math|Float|Lerp 0.0 (Variables|Default|GetHigh%20value) _elevator)) false false))))

(fn ConstructionScript)