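; Auto-turret prop that targets the nearest visible pawn in range and fires bullet bursts from twin barrels.
; Each tick FindTarget runs a sphere overlap and line-of-sight trace, then an incrementer cycles between targeting and firing phases.
; Targeting rotates the top at constant speed; firing checks rate of fire and dot-product alignment.
; Fire uses a DoN loop with delays to alternate left and right socket-spawned BP_Bullets and muzzle flashes.
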(event Custom|Fire
  (bind _turrets_l (Variables|Default|Getturrets_L))
  (bind _turrets_r (Variables|Default|Getturrets_R))
  (bind _returnvalue (Transformation|GetSocketTransform _turrets_l "BulletSocket" "RTS_World"))
  (bind _returnvalue_2 (Transformation|GetSocketTransform _turrets_r "BulletSocket" "RTS_World"))
  ;[1 1 1] the time of the next firing
  (Variables|Quantity|SetLastFireTime (Utilities|Time|GetGameTimeinSeconds))
  (Utilities|FlowControl|Sequence
    (:then_0
      (goto _label Reset))
    (:then_1
      ;[1 1 1] the number of bullets fired per firing
      (Utilities|FlowControl|DoN 3 :!label _label
        (:Exit
          ;[1 1 1] a certain amount of time is delayed between each barrel spawn bullet
          (Game|SpawnActorfromClass "/Game/Props/stationary_turrets/BP_Bullet.BP_Bullet_C" (Math|Transform|MakeTransform (.location _returnvalue) (.rotation _returnvalue) "1.000000,1.000000,1.000000") "Undefined" 0 0)
          (Components|Activation|SetActive (Variables|Default|GetMuzzle_flash_VFX_L) true true)
          ;[1 1 1] Delay between 2 turrets
          (Utilities|FlowControl|Delay 0.2)
          (Game|SpawnActorfromClass "/Game/Props/stationary_turrets/BP_Bullet.BP_Bullet_C" (Math|Transform|MakeTransform (.location _returnvalue_2) (.rotation _returnvalue_2) "1.000000,1.000000,1.000000") "Undefined" 0 0)
          (Components|Activation|SetActive (Variables|Default|GetMuzzle_flash_VFX_R) true true)
          (Utilities|FlowControl|Delay 0.2)
          (goto _label))))))

(event EventBeginPlay
  (Variables|Default|SetTotalCycleDuration (+ (Variables|Default|GetTargetingDuration) (Variables|Default|GetFiringDuration))))

(event Collision|EventActorBeginOverlap
  (params (OtherActor :type Actor%20Object%20Reference)))

(event EventTick
  (params (DeltaSeconds :type Float%20%28single-precision%29))
  ;[1 1 1] rotate the turret and fire after getting a valid Target (a character that is within attack range and not blocked
  (CallFunction|FindTarget)
  (Variables|Quantity|GetTarget
    (:then
      (CallFunction|IncrementUp DeltaSeconds)
      (if (<= (Variables|Default|GetIncrementer) (Variables|Default|GetTotalCycleDuration))
        (if (<= (Variables|Default|GetIncrementer) (Variables|Default|GetTargetingDuration))
          (CallFunction|RotateTop(UpDate) DeltaSeconds)
          (else
            (CallFunction|UpDateFire)))
        (else
          (Variables|Default|SetIncrementer (- (Variables|Default|GetIncrementer) (Variables|Default|GetTotalCycleDuration))))))
    (:else
      (Variables|Default|SetIncrementer 0.0))))

(fn ConstructionScript)

(fn FindTarget
  ;[1 1 1] detect distance: Sets the attack range of the turret
  (LocalVariables|SetBestDistance%28Local%29 (+ (Variables|quantity|GetScanRange) 1.0))
  ;[1 1 1] detect the pawn(Character), and calculate the distance between the turret and Character
  (bind _outactors (Collision|SphereOverlapActors (Transformation|GetActorLocation) (Variables|quantity|GetScanRange) (Utilities|Array|MakeArray "ObjectTypeQuery3") "/Script/Engine.Actor"))
  (for _array_element _outactors
    (bind _output_get (LocalVariables|SetCurentTarget%28Local%29 _array_element))
    (bind _output_get_2 (LocalVariables|SetCurrentDistance%28Local%29 (Transformation|GetDistanceTo _output_get self)))
    (if (or (not (Utilities|IsValid (LocalVariables|GetBestTaget%28Local%29))) (< _output_get_2 (LocalVariables|GetBestDistance%28Local%29)))
      ;[1 1 1] detect whether there is occlusion between the turret and the character, and execute if there is no occlusion. (The turret will not run when there is an obstacle blocking
      (bind _returnvalue (Collision|LineTraceByChannel (Transformation|GetWorldLocation (Variables|Default|GetSMtop_1)) (Transformation|GetActorLocation (LocalVariables|GetCurentTarget%28Local%29)) "TraceTypeQuery1" false (Utilities|Array|MakeArray self (LocalVariables|GetCurentTarget%28Local%29)) "None" false))
      (if (not _returnvalue)
        (LocalVariables|SetBestTaget%28Local%29 (LocalVariables|GetCurentTarget%28Local%29))
        (LocalVariables|SetBestDistance%28Local%29 (LocalVariables|GetCurrentDistance%28Local%29)))))
  (Variables|Quantity|SetTarget (LocalVariables|GetBestTaget%28Local%29)))

(fn RotateTop(UpDate)
  (params (DeltaSeconds :type Float%20%28double-precision%29))
  (bind _output_get (LocalVariables|SetNewRotation (Class|KismetMathLibrary|RInterptoConstant (Transformation|GetWorldRotation (Variables|Default|GetSMtop_1)) (Math|Rotator|FindLookatRotation (Transformation|GetWorldLocation (Variables|Default|GetSMtop_1)) (Transformation|GetActorLocation (Variables|Quantity|GetTarget))) DeltaSeconds (Variables|Quantity|GetRotateSpeed))))
  (Transformation|SetWorldRotation (Variables|Default|GetSMtop_1) (Math|Rotator|MakeRotator (.roll _output_get) (.pitch _output_get) (.yaw _output_get)) false false))

(fn UpDateFire
  (if (> (- (Utilities|Time|GetTimeSeconds) (Variables|Quantity|GetLastFireTime)) (Variables|Quantity|GetRateOfFire))
    (if (>= (Math|Vector|DotProduct (Math|Vector|GetUnitDirection(Vector) (Transformation|GetWorldLocation (Variables|Default|GetSMtop_1)) (Transformation|GetActorLocation (Variables|Quantity|GetTarget))) (Math|Vector|GetForwardVector (Variables|Default|GetSMtop_1))) 0.99)
      (CallFunction|Fire))))

(fn IncrementUp
  (params (DeltaTime :type Float%20%28double-precision%29))
  (Variables|Default|SetIncrementer (+ DeltaTime (Variables|Default|GetIncrementer))))