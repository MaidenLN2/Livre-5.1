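; Laser prop actor that sweeps a beam back and forth, with a coloured impact effect where it hits.
; Each Tick it line-traces on the Camera channel along the Sphere's forward vector, setting the beam end and placing or hiding the impact effect.
; Beam length snaps to blocking hits and otherwise grows at an emission speed up to a cap.
; A Timeline, played from Tick, drives the Sphere's pitch scaled by an angle variable.
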(event EventBeginPlay
  (Effects|Components|ParticleSystem|SetColorParameter (Variables|Default|GetLaserImpact) "Colour" "(R=0.883681,G=0.084649,B=0.000000,A=1.000000)"))

(event Collision|EventActorBeginOverlap
  (params (OtherActor :type Actor%20Object%20Reference)))

(event EventTick
  (params (DeltaSeconds :type Float%20%28single-precision%29))
  (bind _sphere (Variables|Default|GetSphere))
  (bind _returnvalue (Transformation|GetWorldLocation _sphere))
  (Utilities|FlowControl|Sequence
    (:then_0
      (Variables|Default|SetTraceEnd (+ _returnvalue (* (Math|Vector|GetForwardVector _sphere) (Variables|Default|GetDistance))))
      (bind _outhit (Collision|LineTraceByChannel _returnvalue (+ _returnvalue (* (Math|Vector|GetForwardVector _sphere) (Variables|Default|GetDistance))) "TraceTypeQuery2" false 0 "ForOneFrame"))
      (Variables|Default|SetHit (.bblockinghit _outhit))
      (Variables|Default|SetHitLocation (.location _outhit))
      (Effects|Components|ParticleSystem|SetVectorParameter (Variables|Default|GetLaser) "LaserEnd" (select (Variables|Default|GetHit) (Variables|Default|GetHitLocation) (Variables|Default|GetTraceEnd)))
      ;[1 1 1] Set LaserImpact's world location and visibility
      (Rendering|SetVisibility (Variables|Default|GetLaserImpact) (Variables|Default|GetHit) false)
      (Transformation|SetWorldLocation (Variables|Default|GetLaserImpact) (Variables|Default|GetHitLocation) false false)
      (if (Variables|Default|GetHit)
        (Variables|Default|SetDistance (Math|Vector|VectorLength (- (Variables|Default|GetHitLocation) (Transformation|GetWorldLocation (Variables|Default|GetSphere)))))))
    (:then_1
      (if (< (Variables|Default|GetDistance) 5e+03)
        (Variables|Default|SetDistance (+ (Variables|Default|GetDistance) (* DeltaSeconds (Variables|Default|Getspeed_laser_emission))))))
    (:then_2
      ;[1 1 1] Spin back and forth
      (bind _rotation_1 (Timeline|时间轴 Play)
        (:Update
          (Transformation|SetRelativeRotation (Variables|Default|GetSphere) (Math|Rotator|MakeRotator 0.0 (* _rotation_1 (Variables|Default|Getvalu_rotion_angle)) 0.0) false false))))))

(fn ConstructionScript)