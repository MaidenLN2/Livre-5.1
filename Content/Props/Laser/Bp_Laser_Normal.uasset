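; Laser prop that switches on permanently once a pawn enters its scan range, unless it starts visible.
; While active, each tick line-traces forward along a distance that grows at the emission speed up to a cap, shortening to any blocking hit.
; The trace sets the beam's end parameter and moves and shows a red-orange impact effect at hit points, with per-frame debug drawing left on.
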(event EventBeginPlay
  (Rendering|SetVisibility (Variables|Default|GetLaser) (Variables|Default|GetStart%20visible) false)
  (Effects|Components|ParticleSystem|SetColorParameter (Variables|Default|GetLaserImpact) "Colour" "(R=0.883681,G=0.084649,B=0.000000,A=1.000000)"))

(event EventTick
  (params (DeltaSeconds :type Float%20%28single-precision%29))
  (bind _returnvalue (Transformation|GetActorLocation))
  (bind _returnvalue_2 (Collision|SphereOverlapActors (Transformation|GetActorLocation) (Variables|Default|GetScanRange) (Utilities|Array|MakeArray "ObjectTypeQuery3") "/Script/Engine.Actor"))
  (if (or _returnvalue_2 (Variables|Default|GetStart%20visible))
    (bind _output_get (Variables|Default|SetStart%20visible true))
    (Rendering|SetVisibility (Variables|Default|GetLaser) _output_get false)
    (Utilities|FlowControl|Sequence
      (:then_0
        (Variables|Default|SetTraceEnd (+ _returnvalue (* (Transformation|GetActorForwardVector) (Variables|Default|GetDistance))))
        (bind _outhit (Collision|LineTraceByChannel _returnvalue (+ _returnvalue (* (Transformation|GetActorForwardVector) (Variables|Default|GetDistance))) "TraceTypeQuery2" false 0 "ForOneFrame"))
        (Variables|Default|SetHit (.bblockinghit _outhit))
        (Variables|Default|SetHitLocation (.location _outhit))
        (Effects|Components|ParticleSystem|SetVectorParameter (Variables|Default|GetLaser) "LaserEnd" (select (Variables|Default|GetHit) (Variables|Default|GetHitLocation) (Variables|Default|GetTraceEnd)))
        ;[1 1 1] Set LaserImpact's world location and visibility
        (Rendering|SetVisibility (Variables|Default|GetLaserImpact) (Variables|Default|GetHit) false)
        (Transformation|SetWorldLocation (Variables|Default|GetLaserImpact) (Variables|Default|GetHitLocation) false false)
        (if (Variables|Default|GetHit)
          (Variables|Default|SetDistance (Math|Vector|VectorLength (- (Variables|Default|GetHitLocation) (Transformation|GetActorLocation))))))
      (:then_1
        (if (< (Variables|Default|GetDistance) 5e+03)
          (Variables|Default|SetDistance (+ (Variables|Default|GetDistance) (* DeltaSeconds (Variables|Default|Getspeed_laser_emission)))))))))

(fn ConstructionScript)