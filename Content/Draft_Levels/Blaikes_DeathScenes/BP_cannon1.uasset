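; Auto-targeting cannon turret that tracks nearby pawns and calls Fire when aimed at one.
; Each Tick, FindTarget picks the closest pawn in scan range with an unblocked Visibility trace, and the top mesh turns toward it at constant speed.
; UpDateFire checks the fire interval and a dot-product aim threshold before calling Fire.
; Fire is empty here; the BP_Shell spawning and LastFireTime update are disconnected.
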(event Custom|Fire)

(event EventBeginPlay)

(event Collision|EventActorBeginOverlap
  (params (OtherActor :type Actor%20Object%20Reference)))

(event EventTick
  (params (DeltaSeconds :type Float%20%28single-precision%29))
  (CallFunction|FindTarget)
  (Variables|Quantity|GetTarget
    (:then
      (CallFunction|RotateTop(UpDate) DeltaSeconds)
      (CallFunction|UpDateFire))
    (:else)))

(fn ConstructionScript)

(fn FindTarget
  ;[1 1 1] detect distance
  (LocalVariables|SetBestDistance%28Local%29 (+ (Variables|quantity|GetScanRange) 1.0))
  (bind _outactors (Collision|SphereOverlapActors (Transformation|GetActorLocation) (Variables|quantity|GetScanRange) (Utilities|Array|MakeArray "ObjectTypeQuery3") "/Script/Engine.Actor"))
  (for _array_element _outactors
    (bind _output_get (LocalVariables|SetCurentTarget%28Local%29 _array_element))
    (bind _output_get_2 (LocalVariables|SetCurrentDistance%28Local%29 (Transformation|GetDistanceTo _output_get self)))
    (if (or (not (Utilities|IsValid (LocalVariables|GetBestTaget%28Local%29))) (< _output_get_2 (LocalVariables|GetBestDistance%28Local%29)))
      (bind _returnvalue (Collision|LineTraceByChannel (Transformation|GetWorldLocation (Variables|Default|GetSMtop_1)) (Transformation|GetActorLocation (LocalVariables|GetCurentTarget%28Local%29)) "TraceTypeQuery1" false (Utilities|Array|MakeArray self (LocalVariables|GetCurentTarget%28Local%29)) "None" false))
      (if (not _returnvalue)
        (LocalVariables|SetBestTaget%28Local%29 (LocalVariables|GetCurentTarget%28Local%29))
        (LocalVariables|SetBestDistance%28Local%29 (LocalVariables|GetCurrentDistance%28Local%29)))))
  (Variables|Quantity|SetTarget (LocalVariables|GetBestTaget%28Local%29)))

(fn RotateTop(UpDate)
  (params (DeltaSeconds :type Float%20%28double-precision%29))
  (bind _output_get (LocalVariables|SetNewRotation (Class|KismetMathLibrary|RInterptoConstant (Transformation|GetWorldRotation (Variables|Default|GetSMtop_1)) (Math|Rotator|FindLookatRotation (Transformation|GetWorldLocation (Variables|Default|GetSMtop_1)) (Transformation|GetActorLocation (Variables|Quantity|GetTarget))) DeltaSeconds (Variables|Quantity|GetRotateSpeed))))
  (Transformation|SetWorldRotation (Variables|Default|GetSMtop_1) (Math|Rotator|MakeRotator (.roll _output_get) (.pitch _output_get) (.yaw _output_get)) false false))

(fn UpDateFire
  (if (> (- (Utilities|Time|GetTimeSeconds) (Variables|Quantity|GetLastFireTime)) (Variables|Quantity|GetRateOfFire))
    (if (>= (Math|Vector|DotProduct (Math|Vector|GetUnitDirection(Vector) (Transformation|GetWorldLocation (Variables|Default|GetSMtop_1)) (Transformation|GetActorLocation (Variables|Quantity|GetTarget))) (Math|Vector|GetForwardVector (Variables|Default|GetSMtop_1))) 0.99)
      (CallFunction|Fire))))