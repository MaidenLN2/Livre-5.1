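; MovePlat_BP is a moving platform that shuttles its static mesh back and forth between its starting transform and a Destination offset.
; On BeginPlay it stores the mesh's relative location and rotation, scales the timeline's play rate by TravelTimeInSeconds, and starts moving.
; The Animator timeline's alpha interpolates location and rotation.
; Each finish waits PauseTime, then a FlipFlop alternates reverse and forward playback, looping indefinitely.
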(event Custom|StartMovement
  (bind _initpos (Variables|Default|GetInitPos))
  (bind _initrot (Variables|Default|GetInitRot))
  (bind _destination (Variables|Default|GetDestination))
  (bind _alpha (Timeline|Animator Play)
    (:Update
      (Variables|Default|SetLerpAlpha _alpha)
      (Transformation|SetRelativeLocationAndRotation (Variables|Default|GetStaticMesh) (Math|Vector|Lerp(Vector) _initpos (+ _initpos (.location _destination)) (Variables|Default|GetLerpAlpha)) (Math|Rotator|Lerp(Rotator) _initrot (Math|Rotator|CombineRotators _initrot (.rotation _destination)) (Variables|Default|GetLerpAlpha)) false false))
    (:Finished
      (Utilities|FlowControl|Delay (Variables|Default|GetPauseTime))
      (Utilities|FlowControl|FlipFlop
        (:A
          (CallFunction|ReverseMovement))
        (:B
          (CallFunction|StartMovement))))))

(event Custom|ReverseMovement
  (bind _initpos (Variables|Default|GetInitPos))
  (bind _initrot (Variables|Default|GetInitRot))
  (bind _destination (Variables|Default|GetDestination))
  (bind _alpha (Timeline|Animator Reverse)
    (:Update
      (Variables|Default|SetLerpAlpha _alpha)
      (Transformation|SetRelativeLocationAndRotation (Variables|Default|GetStaticMesh) (Math|Vector|Lerp(Vector) _initpos (+ _initpos (.location _destination)) (Variables|Default|GetLerpAlpha)) (Math|Rotator|Lerp(Rotator) _initrot (Math|Rotator|CombineRotators _initrot (.rotation _destination)) (Variables|Default|GetLerpAlpha)) false false))
    (:Finished
      (Utilities|FlowControl|Delay (Variables|Default|GetPauseTime))
      (Utilities|FlowControl|FlipFlop
        (:A
          (CallFunction|ReverseMovement))
        (:B
          (CallFunction|StartMovement))))))

(event EventBeginPlay
  (bind _staticmesh (Variables|Default|GetStaticMesh))
  (bind _returnvalue (Transformation|GetRelativeTransform _staticmesh))
  (Variables|Default|SetInitPos (.location _returnvalue))
  (Variables|Default|SetInitRot (.rotation _returnvalue))
  (Components|Timeline|SetPlayRate (Variables|Default|GetAnimator) (/ 1.0 (Variables|Default|GetTravelTimeInSeconds)))
  (CallFunction|StartMovement))

(event Collision|EventActorBeginOverlap
  (params (OtherActor :type Actor%20Object%20Reference)))

(event EventTick
  (params (DeltaSeconds :type Float%20%28single-precision%29)))

(fn ConstructionScript)